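; Art prop group actor that animates a desk lamp, desk, laptop and flower, and handles focus highlighting.
; Tick drives each start time offset through UpdateAnimLoop, scaled by inverse MPC_Focus IsReality and wrapping to a loop-start frame at 24 fps.
; With IsLoop off, offsets ease linearly to zero, though the laptop's is applied to Desk.
; Focus events toggle MPC_Focus highlight flashing, while highlight events toggle Guitar's custom-depth stencil.
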(event Custom|Focused
  (params (HitComponent :type Primitive%20Component%20Object%20Reference))
  (Utilities|FlowControl|Sequence
    (:then_0
      (Rendering|Material|SetScalarParameterValue "/Game/VFX/MPC_Focus.MPC_Focus" "IsHighlightFlashing" 1.0 :!class /Script/Engine.KismetMaterialLibrary))))

(event Custom|NotFocused
  (Rendering|Material|SetScalarParameterValue "/Game/VFX/MPC_Focus.MPC_Focus" "IsHighlightFlashing" 0.0 :!class /Script/Engine.KismetMaterialLibrary))

(event Custom|Disable%20Heigh%20Light
  (CallFunction|SetCustomStencil (Variables|Default|GetGuitar) 0 false))

(event Custom|Enable%20Heigh%20Light
  (CallFunction|SetCustomStencil (Variables|Default|GetGuitar) 1 true))

(event EventBeginPlay)

(event Collision|EventActorBeginOverlap
  (params (OtherActor :type Actor%20Object%20Reference)))

(event EventTick
  (params (DeltaSeconds :type Float%20%28single-precision%29))
  (if (Variables|Default|GetIsLoop)
    (Utilities|FlowControl|Sequence
      (:then_0
        (bind _output (CallFunction|UpdateAnimLoop 1e+02 5e+01 (Variables|Default|GetLampAnimOffst)))
        (bind _output_get (Variables|Default|SetLampAnimOffst _output))
        (Class|GeometryCacheComponent|SetStartTimeOffset (Variables|Default|GetDesk_Lamp) _output_get))
      (:then_1
        (bind _output_2 (CallFunction|UpdateAnimLoop 1.5e+02 5e+01 (Variables|Default|GetDeskAnimOffset)))
        (bind _output_get_2 (Variables|Default|SetDeskAnimOffset _output_2))
        (Class|GeometryCacheComponent|SetStartTimeOffset (Variables|Default|GetDesk) _output_get_2))
      (:then_2
        (bind _output_3 (CallFunction|UpdateAnimLoop 5e+01 0.0 (Variables|Default|GetLaptopAnimOffset)))
        (bind _output_get_3 (Variables|Default|SetLaptopAnimOffset _output_3))
        (Class|GeometryCacheComponent|SetStartTimeOffset (Variables|Default|GetLaptop) _output_get_3))
      (:then_3
        (bind _output_4 (CallFunction|UpdateAnimLoop 1.8e+02 5e+01 (Variables|Default|GetFlowerAnimOffset)))
        (bind _output_get_4 (Variables|Default|SetFlowerAnimOffset _output_4))
        (Class|GeometryCacheComponent|SetStartTimeOffset (Variables|Default|GetFlower) _output_get_4)))
    (else
      (Utilities|FlowControl|Sequence
        (:then_0
          (bind _output_get_5 (Variables|Default|SetLampAnimOffst (Math|Interpolation|FInterptoConstant (Variables|Default|GetLampAnimOffst) 0.0 (Utilities|Time|GetWorldDeltaSeconds) 0.8)))
          (Class|GeometryCacheComponent|SetStartTimeOffset (Variables|Default|GetDesk_Lamp) _output_get_5))
        (:then_1
          (bind _output_get_6 (Variables|Default|SetDeskAnimOffset (Math|Interpolation|FInterptoConstant (Variables|Default|GetDeskAnimOffset) 0.0 (Utilities|Time|GetWorldDeltaSeconds) 1.2)))
          (Class|GeometryCacheComponent|SetStartTimeOffset (Variables|Default|GetDesk) _output_get_6))
        (:then_2
          (bind _output_get_7 (Variables|Default|SetLaptopAnimOffset (Math|Interpolation|FInterptoConstant (Variables|Default|GetLaptopAnimOffset) 0.0 (Utilities|Time|GetWorldDeltaSeconds) 0.7)))
          (Class|GeometryCacheComponent|SetStartTimeOffset (Variables|Default|GetDesk) _output_get_7))
        (:then_3
          (bind _output_get_8 (Variables|Default|SetFlowerAnimOffset (Math|Interpolation|FInterptoConstant (Variables|Default|GetFlowerAnimOffset) 0.0 (Utilities|Time|GetWorldDeltaSeconds) 1.0)))
          (Class|GeometryCacheComponent|SetStartTimeOffset (Variables|Default|GetFlower) _output_get_8))))))

(fn ConstructionScript)

(fn SetCustomStencil
  (params (Component :type Primitive%20Component%20Object%20Reference) (Value :type Integer) (Enable :type Boolean))
  (Rendering|SetRenderCustomDepth Component Enable)
  (Rendering|SetCustomDepthStencilValue Component Value))

(fn UpdateAnimLoop
  (params (TotalFrames :type Float%20%28double-precision%29) (LoopStartFrames :type Float%20%28double-precision%29) (AnimOffset :type Float%20%28double-precision%29))
  (bind _returnvalue (/ TotalFrames 24.0))
  (bind _returnvalue_2 (Rendering|Material|GetScalarParameterValue "/Game/VFX/MPC_Focus.MPC_Focus" "IsReality" :!class /Script/Engine.KismetMaterialLibrary))
  (LocalVariables|SetFinal (+ AnimOffset (* (Utilities|Time|GetWorldDeltaSeconds) (* (- 1.0 _returnvalue_2) 2.0))))
  (if (> (+ AnimOffset (* (Utilities|Time|GetWorldDeltaSeconds) (* (- 1.0 _returnvalue_2) 2.0))) _returnvalue)
    (LocalVariables|SetFinal (* _returnvalue (/ LoopStartFrames TotalFrames))))
  (return (LocalVariables|GetFinal)))