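; Blueprint that controls looping of the DeskLamp's animation by setting its start time offset.
; The Loop and NotLoop events toggle a flag that lets Tick pass UpdateAnimLoop's result to DeskLamp each frame.
; UpdateAnimLoop converts frames to seconds at 24 fps and resets AnimOffset to the loop start frame when the next step would pass the end.
; The visible graph never increments AnimOffset.
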(event Custom|NotLoop
  (Variables|Default|SetIsLoop_Single false))

(event Custom|Loop
  (Variables|Default|SetIsLoop_Single true))

(event EventBeginPlay)

(event EventTick
  (params (DeltaSeconds :type Float%20%28single-precision%29))
  (if (Variables|Default|GetIsLoop_Single)
    (bind _output (CallFunction|UpdateAnimLoop 1e+02 5e+01))
    (Class|GeometryCacheComponent|SetStartTimeOffset (Variables|Default|GetDesk_Lamp) _output)))

(fn UpdateAnimLoop
  (params (TotalFrames :type Float%20%28double-precision%29) (LoopStartFrames :type Float%20%28double-precision%29))
  (bind _returnvalue (/ TotalFrames 24.0))
  (if (> (+ (Variables|Default|GetAnimOffset) (Utilities|Time|GetWorldDeltaSeconds)) _returnvalue)
    (bind _output_get (Variables|Default|SetAnimOffset (* _returnvalue (/ LoopStartFrames TotalFrames)))))
  (return _output_get))