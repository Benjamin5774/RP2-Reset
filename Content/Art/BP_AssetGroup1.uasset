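; BP_AssetGroup1 is an art asset Blueprint that provides focus highlighting for a Horse component and a helper for looping animation timing.
; Focus events switch a flashing parameter in MPC_Focus, while separate highlight events toggle the horse's custom depth stencil.
; UpdateAnimLoop, not called in this graph, advances a time offset scaled by the inverse of IsReality, wrapping to a loop start frame at 24 fps.
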(event Custom|Focused
  (params (HitComponent :type Primitive%20Component%20Object%20Reference))
  (Utilities|FlowControl|Sequence
    (:then_0
      (Rendering|Material|SetScalarParameterValue "/Game/VFX/MPC_Focus.MPC_Focus" "IsHighlightFlashing" 1.0 :!class /Script/Engine.KismetMaterialLibrary))))

(event Custom|NotFocused
  (Rendering|Material|SetScalarParameterValue "/Game/VFX/MPC_Focus.MPC_Focus" "IsHighlightFlashing" 0.0 :!class /Script/Engine.KismetMaterialLibrary))

(event Custom|Disable%20Heigh%20Light
  (CallFunction|SetCustomStencil (Variables|Default|GetHorse) 0 false))

(event Custom|Enable%20Heigh%20Light
  (CallFunction|SetCustomStencil (Variables|Default|GetHorse) 1 true))

(event Collision|EventActorBeginOverlap
  (params (OtherActor :type Actor%20Object%20Reference)))

(event EventTick
  (params (DeltaSeconds :type Float%20%28single-precision%29)))

(fn ConstructionScript)

(fn SetCustomStencil
  (params (Component :type Primitive%20Component%20Object%20Reference) (Value :type Integer) (Enable :type Boolean))
  (Rendering|SetRenderCustomDepth Component Enable)
  (Rendering|SetCustomDepthStencilValue Component Value))

(fn UpdateAnimLoop
  (params (TotalFrames :type Float%20%28double-precision%29) (LoopStartFrames :type Float%20%28double-precision%29) (AnimOffset :type Float%20%28double-precision%29))
  (bind _returnvalue (/ TotalFrames 24.0))
  (bind _returnvalue_2 (Rendering|Material|GetScalarParameterValue "/Game/VFX/MPC_Focus.MPC_Focus" "IsReality" :!class /Script/Engine.KismetMaterialLibrary))
  (LocalVariables|SetFinal (+ AnimOffset (* (Utilities|Time|GetWorldDeltaSeconds) (* (- 1.0 _returnvalue_2) 2.0))))
  (if (> (+ AnimOffset (* (Utilities|Time|GetWorldDeltaSeconds) (* (- 1.0 _returnvalue_2) 2.0))) _returnvalue)
    (LocalVariables|SetFinal (* _returnvalue (/ LoopStartFrames TotalFrames))))
  (return (LocalVariables|GetFinal)))