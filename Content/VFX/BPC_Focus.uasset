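; Pawn component that detects what the player is looking at, driving focus on target objects and a reaction to seeing a monster.
; BeginPlay caches the owner's camera, GameManager game instance, BP_GameManager actor and first "Monster1"-tagged actor.
; Each Tick, a debug-drawn camera line trace sets IsRightFocused and calls Focused on BP_AssetGroup hits.
; Hitting that monster plays a heartbeat sound every frame; older pause-check and heart-rate effect branches are disconnected.
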(event EventBeginPlay
  (Utilities|FlowControl|Sequence
    (:then_0
      ;[0.15 0.15 0.15 0.5] fov废案
      (bind _aspawn (Utilities|Casting|CastToPawn (Components|GetOwner)))
      (Variables|Default|SetCameraActor (Actor|GetComponentbyClass _aspawn "/Script/Engine.CameraComponent")))
    (:then_1
      ;[0.15 0.15 0.15 0.5] 游戏开始
      (bind _returnvalue (Game|GetGameInstance))
      (bind _asgame_manager (Utilities|Casting|CastToGameManager _returnvalue)
        (:then
          (Variables|Default|SetGame%20Manager _asgame_manager))
        (:CastFailed
          _))
      (bind _returnvalue_2 (Actor|GetActorOfClass "/Game/Parasomnia/Blueprints/BP_GameManager.BP_GameManager_C"))
      (Variables|Default|SetBP%20Game%20Manager _returnvalue_2))
    (:then_2
      (bind _outactors (Actor|GetAllActorswithTag "Monster1"))
      (Variables|Default|SetMosterTagArray (Utilities|Array|Get(acopy) _outactors)))))

(event EventTick
  (params (DeltaSeconds :type Float%20%28single-precision%29))
  (bind _cameraactor (Variables|Default|GetCameraActor))
  (bind _returnvalue (Transformation|GetWorldLocation _cameraactor))
  ;[0.15 0.15 0.15 0.5] 动头检测
  (bind _outhit (Collision|LineTraceByChannel _returnvalue (+ _returnvalue (* (Math|Vector|GetForwardVector _cameraactor) 1e+04)) "TraceTypeQuery1" false 0 "ForOneFrame"))
  (Utilities|FlowControl|Sequence
    (:then_0
      (bind _asbp_asset_group (Utilities|Casting|CastToBP_AssetGroup (.HitActor (Collision|BreakHitResult _outhit)))
        (:then
          ;;[0.15 0.15 0.15 0.5] 看正确物体逻辑
          (Variables|/Game/Parasomnia/Blueprints/GameManager.GameManager_C|SetisRightFocused (Variables|Default|GetGame%20Manager) true)
          (Default|Focused _asbp_asset_group (.HitComponent (Collision|BreakHitResult _outhit))))
        (:CastFailed
          ;;;[0.15 0.15 0.15 0.5] 错误的话
          (Variables|/Game/Parasomnia/Blueprints/GameManager.GameManager_C|SetisRightFocused (Variables|Default|GetGame%20Manager) false))))
    (:then_1
      ;;[0.15 0.15 0.15 0.5] 看到怪物的逻辑
      (bind _asskeletal_mesh_actor (Utilities|Casting|CastToSkeletalMeshActor (.HitActor (Collision|BreakHitResult _outhit))))
      (if (== _asskeletal_mesh_actor (Variables|Default|GetMosterTagArray))
        (Utilities|FlowControl|Sequence
          (:then_0
            (Audio|Components|Audio|Play (Variables|/Game/Parasomnia/Blueprints/BP_GameManager.BP_GameManager_C|GetHeartBeatSound3 (Variables|Default|GetBP%20Game%20Manager)) 0.0)))))))