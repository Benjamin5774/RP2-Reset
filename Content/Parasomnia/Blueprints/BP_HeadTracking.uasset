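; BP_HeadTracking is an unfinished actor prototype, apparently for detecting whether the player looks at objects tagged "Focusable".
; BeginPlay only fetches the player controller and its location without using the result, and Tick is empty.
; Unreached debug nodes print the location, deproject the screen center, and line trace to report focus.
; The deprojection does not feed the trace, whose endpoints are unset, so no head tracking runs.
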(event EventBeginPlay
  (Utilities|FlowControl|Sequence
    (:then_0
      (bind _returnvalue (Game|GetPlayerController 0))
      (Transformation|GetActorLocation _returnvalue))))

(event Collision|EventActorBeginOverlap
  (params (OtherActor :type Actor%20Object%20Reference)))

(event EventTick
  (params (DeltaSeconds :type Float%20%28single-precision%29)))

(fn ConstructionScript)