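; BP_MonsterManager is a stub manager intended to drive monster animation from the game's current monster state.
; On BeginPlay it casts the Game Instance to GameManager, and Tick reads that cast result directly.
; While the game is not paused, Tick polls MonsterState through a sequence of branches.
; Each of the three handled states only prints a debug string, with no animation played yet.
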(event EventBeginPlay
  ;[0.15 0.15 0.15 0.5] 初始化Monster State
  (Utilities|FlowControl|Sequence
    (:then_0
      (bind _returnvalue (Game|GetGameInstance))
      (bind _asgame_manager (Utilities|Casting|CastToGameManager _returnvalue)))))

(event EventTick
  (params (DeltaSeconds :type Float%20%28single-precision%29))
  ;[0.15 0.15 0.15 0.5] 怪物动画管理
  (if (not (Variables|/Game/Parasomnia/Blueprints/GameManager.GameManager_C|GetisPaused (stale EventBeginPlay _asgame_manager)))
    (Utilities|FlowControl|Sequence
      (:then_0
        (if (== (Variables|/Game/Parasomnia/Blueprints/GameManager.GameManager_C|GetmonsterState (stale EventBeginPlay _asgame_manager)) 0)
          (Development|PrintString "PlayerMonster 0")))
      (:then_1
        (if (== (Variables|/Game/Parasomnia/Blueprints/GameManager.GameManager_C|GetmonsterState (stale EventBeginPlay _asgame_manager)) 1)
          (Development|PrintString "PlayerMonster 1")))
      (:then_2
        (if (== (Variables|/Game/Parasomnia/Blueprints/GameManager.GameManager_C|GetmonsterState (stale EventBeginPlay _asgame_manager)) 2)
          (Development|PrintString "PlayerMonster 2"))))))

(fn ConstructionScript)