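; Level manager actor that scripts the VR intro on BeginPlay, from waking in reality through the shift to surrealism and into Level 1.
; Delays sequence BP_AudioManager music fades, MPC_Focus reality and eye-open changes, and the Monster1 reveal, then set GameManager game-instance state.
; Helpers toggle actor visibility and drive VRPawn heartbeat effects, MPC_HeartRate mode and matching sounds.
; The closing guitar highlight is only a PrintString placeholder.
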(event EventBeginPlay
  (Utilities|FlowControl|Sequence
    (:then_0
      ;[0.15 0.15 0.15 0.5] 全局参数
      (bind _returnvalue (Game|GetGameInstance))
      (bind _asgame_manager (Utilities|Casting|CastToGameManager _returnvalue)))
    (:then_1
      ;[0.15 0.15 0.15 0.5] 声音参数
      (bind _returnvalue_2 (Actor|GetActorOfClass "/Game/Parasomnia/Blueprints/BP_AudioManager.BP_AudioManager_C"))
      (Variables|Default|SetAudioManager _returnvalue_2))
    (:then_2
      ;[0.15 0.15 0.15 0.5] 心跳设置为不可见, 怪物设置不可见
      (CallFunction|SetHeartRateEffect false)
      (bind _outactors (Actor|GetAllActorswithTag "Monster1"))
      (CallFunction|SetObjectVisible false (Utilities|Array|Get(acopy) _outactors)))
    (:then_5
      ;[0.15 0.15 0.15 0.5] 进入场景->现实->第一次超现实
      (Rendering|Material|SetScalarParameterValue "/Game/VFX/MPC_Focus.MPC_Focus" "IsReality" 1.0 :!class /Script/Engine.KismetMaterialLibrary)
      (Utilities|FlowControl|Delay 5.0)
      (Utilities|FlowControl|Sequence
        (:then_0
          ;;[0.15 0.15 0.15 0.5] 淡出主菜单BGM，淡入醒来BGM
          (Audio|Components|Audio|FadeOut (Variables|/Game/Parasomnia/Blueprints/BP_AudioManager.BP_AudioManager_C|GetMainMenu (Variables|Default|GetAudioManager)) 1.0 0.0 "Linear" :!class /Script/Engine.AudioComponent)
          (Utilities|FlowControl|Delay 3.0)
          (Audio|Components|Audio|FadeIn (Variables|/Game/Parasomnia/Blueprints/BP_AudioManager.BP_AudioManager_C|GetWakeUpToSurrealism (Variables|Default|GetAudioManager)) 1.0 1.0 0.0 "Linear" :!class /Script/Engine.AudioComponent)
          (Utilities|FlowControl|Sequence
            (:then_0
              (Variables|/Game/Parasomnia/Blueprints/GameManager.GameManager_C|SetgameStart _asgame_manager true))
            (:then_1
              (Utilities|FlowControl|Delay 3.0)
              (Rendering|Material|SetScalarParameterValue "/Game/VFX/MPC_Focus.MPC_Focus" "IsReality" 0.0 :!class /Script/Engine.KismetMaterialLibrary)
              (Utilities|FlowControl|Sequence
                (:then_0
                  (CallFunction|SetObjectVisible true (Utilities|Array|Get(acopy) _outactors))
                  (CallFunction|SetHeartRateEffect true))
                (:then_1
                  ;;[0.15 0.15 0.15 0.5] Clock音效
                  (CallFunction|PlayBGM (Variables|/Game/Parasomnia/Blueprints/BP_AudioManager.BP_AudioManager_C|GetClock (Variables|Default|GetAudioManager)) 1.0 5.0)
                  (CallFunction|SetHeartRateEffect false)
                  (Utilities|FlowControl|Sequence
                    (:then_0
                      ;[0.15 0.15 0.15 0.5] 进入关卡1，设置怪物动画一阶段，心跳设置为三阶段
                      (Variables|/Game/Parasomnia/Blueprints/GameManager.GameManager_C|SetisLevel1 _asgame_manager true)
                      (Variables|/Game/Parasomnia/Blueprints/GameManager.GameManager_C|SetmonsterState _asgame_manager 0)
                      (Variables|/Game/Parasomnia/Blueprints/GameManager.GameManager_C|SetheartbeatState _asgame_manager 2))
                    (:then_1
                      ;[0.15 0.15 0.15 0.5] 等一会儿高亮吉他
                      (Utilities|FlowControl|Delay 3.0)
                      (Development|PrintString "吉他亮吉他亮吉他亮吉他亮吉他亮"))))))))
        (:then_1
          ;;[0.15 0.15 0.15 0.5] 睁眼特效
          (bind _newtrack_0 (Timeline|Timeline Play)
            (:Update
              (Rendering|Material|SetScalarParameterValue "/Game/VFX/MPC_Focus.MPC_Focus" "IsEyeOpen" _newtrack_0 :!class /Script/Engine.KismetMaterialLibrary))))))))

(event EventTick
  (params (DeltaSeconds :type Float%20%28single-precision%29)))

(fn ConstructionScript)

(fn SetObjectVisible
  (params (Visible :type Boolean) (TargetObject :type Actor%20Object%20Reference))
  (Rendering|SetActorHiddenInGame TargetObject (not Visible))
  (Collision|SetActorEnableCollision TargetObject Visible)
  (Actor|Tick|SetActorTickEnabled TargetObject Visible))

(fn SetHeartRateSound
  (params (Visible :type Boolean) (HeartBeatState :type Integer))
  (Utilities|FlowControl|Sequence
    (:then_1
      (if (== HeartBeatState 0)
        (if Visible
          (Audio|Components|Audio|Play (Variables|Default|GetHeartBeatSound1) 0.0))))
    (:then_2
      (if (== HeartBeatState 1)
        (if Visible
          (Audio|Components|Audio|Play (Variables|Default|GetHeartBeatSound2) 0.0))))
    (:then_3
      (if (== HeartBeatState 2)
        (if Visible
          (Audio|Components|Audio|Play (Variables|Default|GetHeartBeatSound3) 0.0))))
    (:then_4
      (if (== HeartBeatState 3)
        (if Visible
          (Utilities|FlowControl|Sequence
            (:then_0
              (Audio|Components|Audio|Play (Variables|Default|GetHeartBeatSound4) 0.0))
            (:then_1
              (Audio|Components|Audio|Play (Variables|Default|GetHeartBeatSound4Noise) 0.0))))))))

(fn SetHeartRateEffect
  (params (Visible :type Boolean) (HeartBeatState :type Integer))
  (bind _returnvalue (not Visible))
  (Utilities|FlowControl|Sequence
    (:then_0
      (bind _returnvalue_2 (Actor|GetActorOfClass "/Game/VRTemplate/Blueprints/VRPawn.VRPawn_C"))
      (Utilities|FlowControl|Sequence
        (:then_0
          (Development|SetHiddeninGame (Variables|/Game/VRTemplate/Blueprints/VRPawn.VRPawn_C|GetHeartRateEffect3 _returnvalue_2) _returnvalue false))
        (:then_1
          (Development|SetHiddeninGame (Variables|/Game/VRTemplate/Blueprints/VRPawn.VRPawn_C|GetHeartRateEffect2 _returnvalue_2) _returnvalue false))
        (:then_2
          (Development|SetHiddeninGame (Variables|/Game/VRTemplate/Blueprints/VRPawn.VRPawn_C|GetHeartRateEffect1 _returnvalue_2) _returnvalue false))
        (:then_3
          (Development|SetHiddeninGame (Variables|/Game/VRTemplate/Blueprints/VRPawn.VRPawn_C|GetHeartRateEffect _returnvalue_2) _returnvalue false))))
    (:then_1
      (if (== HeartBeatState 0)
        (if Visible
          (Rendering|Material|SetScalarParameterValue "/Game/MPC_HeartRate.MPC_HeartRate" "Mode123" 0.0 :!class /Script/Engine.KismetMaterialLibrary)
          (Audio|Components|Audio|Play (Variables|Default|GetHeartBeatSound1) 0.0))))
    (:then_2
      (if (== HeartBeatState 1)
        (if Visible
          (Rendering|Material|SetScalarParameterValue "/Game/MPC_HeartRate.MPC_HeartRate" "Mode123" 1.0 :!class /Script/Engine.KismetMaterialLibrary)
          (Audio|Components|Audio|Play (Variables|Default|GetHeartBeatSound2) 0.0))))
    (:then_3
      (if (== HeartBeatState 2)
        (if Visible
          (Rendering|Material|SetScalarParameterValue "/Game/MPC_HeartRate.MPC_HeartRate" "Mode123" 2.0 :!class /Script/Engine.KismetMaterialLibrary)
          (Audio|Components|Audio|Play (Variables|Default|GetHeartBeatSound3) 0.0))))
    (:then_4
      (if (== HeartBeatState 3)
        (if Visible
          (Rendering|Material|SetScalarParameterValue "/Game/MPC_HeartRate.MPC_HeartRate" "Mode123" 3.0 :!class /Script/Engine.KismetMaterialLibrary)
          (Utilities|FlowControl|Sequence
            (:then_0
              (Audio|Components|Audio|Play (Variables|Default|GetHeartBeatSound4) 0.0))
            (:then_1
              (Audio|Components|Audio|Play (Variables|Default|GetHeartBeatSound4Noise) 0.0))))))
    (:then_5
      (if (not Visible)
        (Audio|Components|Audio|Stop (Variables|Default|GetHeartBeatSound1))))
    (:then_6
      (if (not Visible)
        (Audio|Components|Audio|Stop (Variables|Default|GetHeartBeatSound2))))
    (:then_7
      (if (not Visible)
        (Audio|Components|Audio|Stop (Variables|Default|GetHeartBeatSound3))))
    (:then_8
      (if (not Visible)
        (Utilities|FlowControl|Sequence
          (:then_0
            (Audio|Components|Audio|Stop (Variables|Default|GetHeartBeatSound4)))
          (:then_1
            (Audio|Components|Audio|Stop (Variables|Default|GetHeartBeatSound4Noise))))))))

(fn PlayBGM
  (params (NewSound :type Audio%20Component%20Object%20Reference) (FadeInTime :type Float%20%28double-precision%29) (During :type Float%20%28double-precision%29))
  (Audio|Components|Audio|FadeIn NewSound FadeInTime 1.0 0.0 "Linear" :!class /Script/Engine.AudioComponent)
  (Audio|Components|Audio|FadeOut NewSound During 0.0 "Linear" :!class /Script/Engine.AudioComponent))