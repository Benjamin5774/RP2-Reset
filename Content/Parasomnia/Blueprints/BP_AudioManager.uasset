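; BP_AudioManager is an audio manager Blueprint with functions meant for fading background music in and out.
; BGMFadeIn checks that NewSound is valid, then fades in MainMenu without using NewSound further.
; BGMFadeOut makes the same check but leads into an empty sequence, so it fades nothing.
; The event graph and construction script contain no active logic.
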(event EventBeginPlay)

(event Collision|EventActorBeginOverlap
  (params (OtherActor :type Actor%20Object%20Reference)))

(event EventTick
  (params (DeltaSeconds :type Float%20%28single-precision%29)))

(fn ConstructionScript)

(fn BGMFadeOut
  (if (Utilities|IsValid (Variables|Default|GetNewSound))
    (Utilities|FlowControl|Sequence)))

(fn BGMFadein
  (if (Utilities|IsValid (Variables|Default|GetNewSound))
    (Utilities|FlowControl|Sequence
      (:then_2
        ;[0.15 0.15 0.15 0.5] 淡入
        (Audio|Components|Audio|FadeIn (Variables|Default|GetMainMenu) 1.0 1.0 0.0 "Linear" :!class /Script/Engine.AudioComponent)))))