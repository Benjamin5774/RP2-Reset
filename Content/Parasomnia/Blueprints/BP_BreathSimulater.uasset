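; VR breathing simulator that turns motion controller height into a breath value to pull the player back toward reality.
; The controller's Z, calibrated at BeginPlay or with E, becomes a clamped value each active Tick, driving the breath bar, BPBreathing and BreathIn/BreathOut playback.
; Each peak-to-trough cycle counts as a breath, raising MPC_Focus "IsReality" in steps while a GameManager right-focus flag is set.
; Hand-button breathing logic is disconnected.
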(event Input|EnhancedActionEvents|EnhancedInputActionIA_Breath_left
  (params (ActionValue :type Boolean) (ElapsedSeconds :type Float%20%28double-precision%29) (TriggeredSeconds :type Float%20%28double-precision%29) (InputAction :type Input%20Action%20Object%20Reference :default "/Game/Parasomnia/Blueprints/IA_Breath_left.IA_Breath_left"))
  ;[0.15 0.15 0.15 0.5] 左手输入检测 Left-hand input detection
)

(event Input|EnhancedActionEvents|EnhancedInputActionIA_Hand_Grasp_Right
  (params (ActionValue :type Float%20%28double-precision%29) (ElapsedSeconds :type Float%20%28double-precision%29) (TriggeredSeconds :type Float%20%28double-precision%29) (InputAction :type Input%20Action%20Object%20Reference :default "/Game/VRTemplate/Input/Actions/Hands/IA_Hand_Grasp_Right.IA_Hand_Grasp_Right"))
  ;[0.15 0.15 0.15 0.5] 右手输入检测 Right-hand input detection
)

(event EventBeginPlay
  ;[0.15 0.15 0.15 0.5] 游戏开始 Game Start
  (Utilities|FlowControl|Sequence
    (:then_0
      ;;[0.15 0.15 0.15 0.5] 获取呼吸条 UI Get the breathing bar UI
      (bind _returnvalue (Game|Player|GetPlayerPawn 0))
      (bind _asvrpawn (Utilities|Casting|CastToVRPawn _returnvalue))
      (Utilities|FlowControl|Sequence
        (:then_0
          ;;[0.15 0.15 0.15 0.5] 获取z轴 Get the z-axis
          (bind _returnvalue_2 (Actor|GetComponentbyClass _asvrpawn "/Script/HeadMountedDisplay.MotionControllerComponent"))
          (bind _returnvalue_3 (Transformation|GetWorldLocation _returnvalue_2))
          (Variables|Default|Set%20InitialZ (.Z (Math|Vector|BreakVector _returnvalue_3))))
        (:then_1
          (bind _returnvalue_4 (UserInterface|GetUserWidgetObject (Variables|/Game/VRTemplate/Blueprints/VRPawn.VRPawn_C|GetBreathWidget _asvrpawn)))
          (bind _aswbp_breath_bar (Utilities|Casting|CastToWBP_BreathBar _returnvalue_4))
          (Variables|Default|SetWBPRef _aswbp_breath_bar))))
    (:then_1
      ;;[0.15 0.15 0.15 0.5] 注册输入映射 Registering Input Mappings
      (bind _returnvalue_5 (Game|GetPlayerController 0))
      (Input|AddMappingContext (PlayerController|LocalPlayerSubsystems|GetEnhancedInputLocalPlayerSubsystem _returnvalue_5) (Variables|Default|GetIMC_Breath) 5 "(bIgnoreAllPressedKeysUntilRelease=True,bForceImmediately=False,bNotifyUserSettings=False)"))
    (:then_2
      ;;[0.15 0.15 0.15 0.5] 初始化呼吸数值 Initialize breathing value
      (Variables|Default|SetBreathValue 0.0))
    (:then_3
      ;[0.15 0.15 0.15 0.5] 判断游戏开始
      (bind _returnvalue_6 (Game|GetGameInstance))
      (bind _asgame_manager (Utilities|Casting|CastToGameManager _returnvalue_6)))))

(event EventTick
  (params (DeltaSeconds :type Float%20%28single-precision%29))
  (bind __initialz (Variables|Default|Get%20InitialZ))
  ;[0.15 0.15 0.15 0.5] 呼吸数值 Breathing value
  ;[0.15 0.15 0.15 0.5] 判断游戏开始
  (if (Variables|/Game/Parasomnia/Blueprints/GameManager.GameManager_C|GetgameStart (stale EventBeginPlay _asgame_manager))
    (if (not (Variables|/Game/Parasomnia/Blueprints/GameManager.GameManager_C|GetisPaused (stale EventBeginPlay _asgame_manager)))
      (Utilities|FlowControl|Sequence
        (:then_0
          ;;[0.15 0.15 0.15 0.5] 判断有没有按住 Determine whether the
          (if (not (Variables|Default|GetbIsInhaling))
            (bind _output_get (Variables|Default|SetBreathValue (stale _returnvalue_5) :!label _label))
            (if (<= _output_get 0.0)
              (Audio|Components|Audio|Play (Variables|Default|GetBreathIn) 0.0)
              (else
                (bind _returnvalue (Game|Player|GetPlayerPawn 0))
                (Utilities|FlowControl|Sequence
                  (:then_0
                    ;[0.15 0.15 0.15 0.5] 更新UI Update UI
                    (bind _asvrpawn (Utilities|Casting|CastToVRPawn _returnvalue))
                    (bind _returnvalue_2 (UserInterface|GetUserWidgetObject (Variables|/Game/VRTemplate/Blueprints/VRPawn.VRPawn_C|GetBreathWidget _asvrpawn)))
                    (bind _aswbp_breath_bar (Utilities|Casting|CastToWBP_BreathBar _returnvalue_2))
                    (Variables|/Game/Parasomnia/UI/WBP_BreathBar.WBP_BreathBar_C|SetBreathPercent _aswbp_breath_bar _output_get))
                  (:then_1
                    (Audio|Components|Audio|Play (Variables|Default|GetBreathOut) 0.0)))))))
        (:then_1
          (Development|PrintString "HelloHelloHelloHelloHelloHelloHello" (Math|Boolean|ORBoolean (Variables|/Game/Parasomnia/Blueprints/GameManager.GameManager_C|GetisJITARightFocused (stale EventBeginPlay _asgame_manager)) (Variables|/Game/Parasomnia/Blueprints/GameManager.GameManager_C|GetisSIMARightFocused (stale EventBeginPlay _asgame_manager)) (Variables|/Game/Parasomnia/Blueprints/GameManager.GameManager_C|GetisSHALOURightFocused (stale EventBeginPlay _asgame_manager)))))
        (:then_2
          ;[0.15 0.15 0.15 0.5] 外接呼吸设备 External respiratory equipment
          (bind _returnvalue_3 (Game|Player|GetPlayerPawn 0))
          (bind _asvrpawn_2 (Utilities|Casting|CastToVRPawn _returnvalue_3))
          (bind _returnvalue_4 (Actor|GetComponentbyClass _asvrpawn_2 "/Script/HeadMountedDisplay.MotionControllerComponent"))
          (Utilities|FlowControl|Sequence
            (:then_0
              (Development|PrintString (Utilities|String|ToString(Vector) (Transformation|GetWorldLocation _returnvalue_4)))
              (bind _z (Math|Vector|BreakVector (Transformation|GetWorldLocation _returnvalue_4)))
              (bind _returnvalue_5 (Math|Float|Clamp(Float) (/ (- _z (- __initialz 0.1)) (Variables|Default|GetMap%20Range))))
              (Utilities|FlowControl|Sequence
                (:then_0
                  (bind _output_get_2 (Variables|Default|SetBreathValue _returnvalue_5))
                  (bind _returnvalue_6 (Game|Player|GetPlayerPawn 0))
                  (Utilities|FlowControl|Sequence))
                (:then_1
                  (goto _label))
                (:then_2
                  ;[0.15 0.15 0.15 0.5] 呼吸效果 Breathing effect
                  (Variables|/Game/VFX/BP_Breathing.BP_Breathing_C|SetTargetBreathingValue (Variables|Default|GetBP_Breathing) _returnvalue_5))))
            (:then_1
              (Development|PrintString (Utilities|String|ToString(Float) __initialz)))))
        (:then_3
          (Development|PrintString (Utilities|String|ToString(Float) (stale _output_get_3))))
        (:then_4
          ;[0.15 0.15 0.15 0.5] 返回现实逻辑 Return to real logic
          ;;[0.15 0.15 0.15 0.5] 吸气达到阈值 Inspiratory threshold reached
          (if (>= (Variables|Default|GetBreathValue) 0.8)
            (Variables|Default|SetbWasAtPeak true)))
        (:then_6
          ;;[0.15 0.15 0.15 0.5] 达到阈值后呼气 Exhale after reaching threshold
          (if (and (Variables|Default|GetbWasAtPeak) (<= (Variables|Default|GetBreathValue) 0.1))
            (Variables|Default|SetBeathCount (Math|Float|Truncate (+ (Variables|Default|GetBeathCount) 1)))
            (Variables|Default|SetbWasAtPeak false)
            ;;;[0.15 0.15 0.15 0.5] 每次增加三分之一的现实(盯着才能触发) Increasing reality by one third each time
            (if (Math|Boolean|ORBoolean (Variables|/Game/Parasomnia/Blueprints/GameManager.GameManager_C|GetisJITARightFocused (stale EventBeginPlay _asgame_manager)) (Variables|/Game/Parasomnia/Blueprints/GameManager.GameManager_C|GetisSIMARightFocused (stale EventBeginPlay _asgame_manager)) (Variables|/Game/Parasomnia/Blueprints/GameManager.GameManager_C|GetisSHALOURightFocused (stale EventBeginPlay _asgame_manager)))
              (if (<= (Variables|Default|GethowReal) 1.02)
                (bind _output_get_3 (Variables|Default|SethowReal (+ (Variables|Default|GethowReal) 0.34)))
                (Utilities|FlowControl|Sequence
                  (:then_0
                    (Rendering|Material|SetScalarParameterValue "/Game/VFX/MPC_Focus.MPC_Focus" "IsReality" _output_get_3 :!class /Script/Engine.KismetMaterialLibrary)))))))
        (:then_7
          (Development|PrintString (Utilities|String|ToString(Boolean) (Variables|Default|GetbWasAtPeak))))
        (:then_8
          (Development|PrintString (Utilities|String|ToString(Integer) (Variables|Default|GetBeathCount))))
        (:then_9
          (Development|PrintString (Utilities|String|ToString(Float) _output_get_2)))))))

(event Input|KeyboardEvents|E
  (params (Key :type Key%20Structure :default "None"))
  ;[0.15 0.15 0.15 0.5] 游戏开始 Game Start
  ;;[0.15 0.15 0.15 0.5] 获取z轴 Get the z-axis
  (:Pressed
    (bind _returnvalue (Actor|GetComponentbyClass (stale EventBeginPlay _asvrpawn) "/Script/HeadMountedDisplay.MotionControllerComponent"))
    (bind _returnvalue_2 (Transformation|GetWorldLocation _returnvalue))
    (Variables|Default|Set%20InitialZ (.Z (Math|Vector|BreakVector _returnvalue_2)))))

(fn ConstructionScript)