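; BP_Heartbeat is an actor that holds a HeartRate value for the game.
; SetHeartRate, IncreaseHeartRate and DecreaseHearRate overwrite or offset the value directly, with no clamping.
; Tick prints the current rate as debug text every frame, and nothing else in the graphs reacts to it.
; An unconnected debug snippet reads IsReality from the MPC_Focus material parameter collection but never runs.
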(event EventBeginPlay)

(event Collision|EventActorBeginOverlap
  (params (OtherActor :type Actor%20Object%20Reference)))

(event EventTick
  (params (DeltaSeconds :type Float%20%28single-precision%29))
  (Utilities|FlowControl|Sequence
    (:then_0
      (Development|PrintString (Utilities|String|ToString(Text) (Utilities|Text|FormatText "Heart Rate = {HeartRate}" (Variables|Default|GetHeartRate)))))))

(fn ConstructionScript)

(fn SetHeartRate
  (params (MyHeartRate :type Float%20%28double-precision%29))
  (Variables|Default|SetHeartRate MyHeartRate))

(fn IncreaseHeartRate
  (params (IncreaseValue :type Float%20%28double-precision%29))
  (Variables|Default|SetHeartRate (+ IncreaseValue (Variables|Default|GetHeartRate))))

(fn DecreaseHearRate
  (params (DecreaseValue :type Float%20%28double-precision%29))
  (Variables|Default|SetHeartRate (- (Variables|Default|GetHeartRate) DecreaseValue)))